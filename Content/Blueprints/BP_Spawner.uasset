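; Enemy spawner actor that places a single BP_Enemy at a random reachable navigation point around itself when play begins.
; After spawning, it shuffles its Names and Mesh arrays and reassigns Materials to itself, printing debug messages along the way.
; None of these arrays are applied to the spawned enemy, and a dynamic material instance node is left unconnected.
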(event `self.ReceiveBeginPlay`
  (`|SpawnActorFromClass` "/Game/ThirdPerson/Blueprints/BP_Enemy.BP_Enemy_C" (`KismetMathLibrary.MakeTransform` (`NavigationSystemV1.K2_GetRandomReachablePointInRadius` (`self.K2_GetActorLocation`) 5000.0 null null)) "Undefined" "MultiplyWithRoot" null null)
  (`KismetSystemLibrary.PrintString` "I got spawn")
  (`KismetArrayLibrary.Array_Shuffle` (`self.Names`))
  (`KismetSystemLibrary.PrintString` "I am getting a name")
  (`KismetArrayLibrary.Array_Shuffle` (`self.Mesh`))
  (set `self.Materials` (`self.Materials`))
  (`KismetSystemLibrary.PrintString` "I am getting a material"))

(fn `UserConstructionScript`)