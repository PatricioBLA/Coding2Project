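; BP_Door1 is a key-locked door that lowers when the player gets near while holding at least one key.
; A Sphere overlap casts to BP_ThirdPersonCharacter and checks TotalKeys, then a DoOnce spends one key and plays a Timeline.
; The Timeline drives a Lerp on the Door's relative Z to slide it down, and an unconnected MoveComponentTo node is left unused.
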(event `self.Sphere.OnComponentBeginOverlap`
  (params (OverlappedComponent :type "PrimitiveComponent Object Reference") (OtherActor :type "Actor Object Reference") (OtherComp :type "PrimitiveComponent Object Reference") (OtherBodyIndex :type Integer) (bFromSweep :type Boolean) (SweepResult :type "HitResult Structure (by ref)"))
  (bind _asbp_third_person_character (cast `/Game/ThirdPerson/Blueprints/BP_ThirdPersonCharacter` OtherActor))
  (`KismetSystemLibrary.PrintString` "I see player")
  (if (> (`/Game/ThirdPerson/Blueprints/BP_ThirdPersonCharacter.Total Keys` _asbp_third_person_character) 0)
    (`/Engine/EditorBlueprintResources/StandardMacros.DoOnce` false
      (:`Completed`
        (`/Engine/EditorBlueprintResources/StandardMacros.DecrementInt` (`/Game/ThirdPerson/Blueprints/BP_ThirdPersonCharacter.Total Keys` _asbp_third_person_character) ; Reduce la cantidad de llaves
          (:`  `
            (bind (_direction _newtrack_0) (`Timeline|Timeline`)
              (:`Update`
                (`SceneComponent.K2_SetRelativeLocation` (`self.Door`) (`KismetMathLibrary.MakeVector` 0.0 0.0 (`KismetMathLibrary.Lerp` 150.0 -140.0 _newtrack_0)) false false)))))))))

(fn `UserConstructionScript`)