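; BP_ElementalBarrier is a barrier that lets the third-person character through when its elemental type matches the barrier's own.
; On begin play, a switch on the element writes the type name to a text render, with only the Fire case wired.
; An overlap on the collision box casts to BP_ThirdPersonCharacter and, on a match, disables the Barrier's collision, which nothing here re-enables.
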(event `self.ReceiveBeginPlay`
  (switch `/Game/Blueprints/E_ElementalType` (`self.ElementalType`)
    (:`NewEnumerator1`
      (`TextRenderComponent.K2_SetText` (`self.TextRender`) (`KismetSystemLibrary.MakeLiteralText` (`KismetTextLibrary.Conv_ByteToText` (`self.ElementalType`)))))))

(event `self.Collition Box.OnComponentBeginOverlap`
  (params (OverlappedComponent :type "PrimitiveComponent Object Reference") (OtherActor :type "Actor Object Reference") (OtherComp :type "PrimitiveComponent Object Reference") (OtherBodyIndex :type Integer) (bFromSweep :type Boolean) (SweepResult :type "HitResult Structure (by ref)"))
  (bind _asbp_third_person_character (cast `/Game/ThirdPerson/Blueprints/BP_ThirdPersonCharacter` OtherActor))
  (if (`|EnumEquality` (`/Game/ThirdPerson/Blueprints/BP_ThirdPersonCharacter.ElemetalType` _asbp_third_person_character) (`self.ElementalType`))
    (`PrimitiveComponent.SetCollisionEnabled` (`self.Barrier`) "NoCollision")))

(fn `UserConstructionScript`)