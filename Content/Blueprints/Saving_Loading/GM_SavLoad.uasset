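; Game mode that handles saving and loading player stats, currently stamina, through an SG_player_Stats save object.
; BeginPlay loads the "PlayerSave" slot or creates a new save object when none exists.
; Loaded stamina targets BP_ThirdPersonCharacter, but the cast takes the player controller rather than the pawn.
; SavePlayerStats writes the object to an empty slot name, not "PlayerSave", without first copying current stamina.
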(event `self.ReceiveBeginPlay`
  (`KismetSystemLibrary.PrintString` "Loading the SavLoad Game Mode" true true (struct :`R` 1.0 :`G` 0.417934 :`A` 1.0))
  (`self.Load Player Stats`))

(event `Load Player Stats`
  (bind _returnvalue (`GameplayStatics.DoesSaveGameExist` "PlayerSave"))
  (if _returnvalue
    (bind _returnvalue_2 (`GameplayStatics.LoadGameFromSlot` "PlayerSave"))
    (bind _assg_player_stats (cast `/Game/Blueprints/Saving_Loading/SG_player_Stats` _returnvalue_2))
    (set `self.SG_PlayerStats` _assg_player_stats)
    (bind _asbp_third_person_character (cast `/Game/ThirdPerson/Blueprints/BP_ThirdPersonCharacter` (`GameplayStatics.GetPlayerController` 0)))
    (set `/Game/ThirdPerson/Blueprints/BP_ThirdPersonCharacter.Stamina` (`/Game/Blueprints/Saving_Loading/SG_player_Stats.Stamina` (`self.SG_PlayerStats`)) _asbp_third_person_character) ; The Player Stamina
    (`KismetSystemLibrary.PrintString` "Playerstats have been loaded" true true (struct :`R` 1.0 :`G` 0.89829 :`A` 1.0) 8.0)
    (else
      (bind _returnvalue_3 (`GameplayStatics.CreateSaveGameObject` "/Game/Blueprints/Saving_Loading/SG_player_Stats.SG_player_Stats_C"))
      (set `self.SG_PlayerStats` _returnvalue_3))))

(event `Save Player Stats`
  (bind _returnvalue (`GameplayStatics.SaveGameToSlot` (`self.SG_PlayerStats`)))
  (if _returnvalue
    (`KismetSystemLibrary.PrintText` "Player Stars Written to Save Game File" true true (struct :`R` 0.634554 :`G` 1.0 :`A` 1.0) 5.0)
    (else
      (`KismetSystemLibrary.PrintText` "Player Stars Could not be Written to Save Game File" true true (struct :`R` 1.0 :`B` 0.049839 :`A` 1.0) 5.0))))

(fn `UserConstructionScript`)