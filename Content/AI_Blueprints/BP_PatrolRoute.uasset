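; BP_PatrolRoute is a patrol route actor that supplies world-space waypoints along its spline, likely for AI.
; GetPatrolPointLocation steps PatrolIndex by Direction, flipping Direction at the spline's ends for back-and-forth movement, and returns that point's location.
; The upper check compares against the point count, so the index can pass the last point, and the lower branch skips the location return.
; A simpler direction-flip alternative is left unconnected.
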(fn `GetPatrolPointLocation`
  (returns (Location :type "Vector Structure"))
  (set `self.Patrol Index` (+ (`self.Patrol Index`) (`self.Direction`))) ; so go "next" point
  (if (>= (`self.Patrol Index`) (`SplineComponent.GetNumberOfSplinePoints` (`self.Spline`)))
    (set `self.Direction` -1)
    (return (`SplineComponent.GetLocationAtSplinePoint` (`self.Spline`) (`self.Patrol Index`) "World"))
    (elif (<= (`self.Patrol Index`) 0)
      (set `self.Direction` 1)
      (else
        (return (`SplineComponent.GetLocationAtSplinePoint` (`self.Spline`) (`self.Patrol Index`) "World"))))))

(fn `UserConstructionScript`)